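; Player character for an auto-runner that advances along world X at a capped, accelerating speed, with lateral position clamped to a lane.
; Tick counts down timers, sweeps the forward move, box-traces for "GroundBox" actors and reloads the level after a fall.
; Landing and leaving-ground transitions drive jump buffering and coyote time; input also triggers a cooldown-limited directional launch dash.
; The obstacle collision branch is an empty stub.
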(event EventBeginPlay
  (Variables|Default|SetCurrentAutoMovementSpeed (Variables|Default|GetBaseAutoMovementSpeed)))

(event EventTick
  (params (DeltaSeconds :type Float%20%28single-precision%29))
  (bind _returnvalue (Transformation|GetActorLocation))
  (bind _returnvalue_2 (Transformation|GetActorLocation))
  (bind _returnvalue_3 (+ _returnvalue "0, 0,-30.000000"))
  (Utilities|FlowControl|Sequence
    (:then_0
      ;[0.1429 0.8385 0.009425 1 45] TIMERS
      (Variables|Default|SetDashCooldownTimer (Math|Float|Clamp(Float) (- (Variables|Default|GetDashCooldownTimer) (Utilities|Time|GetWorldDeltaSeconds)) 0.0 1e+02))
      (Variables|Default|SetCurrentAutoMovementSpeed (Math|Float|Clamp(Float) (+ (Variables|Default|GetCurrentAutoMovementSpeed) (* (Variables|Default|GetAutoMovementSpeedMultiplicator) (Utilities|Time|GetWorldDeltaSeconds))) 0.0 (Variables|Default|GetMaxCurrentMovementSpeed)))
      (Variables|Default|SetJumpBufferingTimer (Math|Float|Clamp(Float) (- (Variables|Default|GetJumpBufferingTimer) (Utilities|Time|GetWorldDeltaSeconds)) 0.0 1e+02))
      (Variables|Default|SetCoyoteTimer (Math|Float|Clamp(Float) (- (Variables|Default|GetCoyoteTimer) (Utilities|Time|GetWorldDeltaSeconds)) 0.0 1e+02)))
    (:then_1
      ;[1 1 1 1 45] AUTO MOVEMENT
      (bind _sweephitresult (Transformation|SetActorLocation (Math|Vector|MakeVector (+ (Variables|Default|GetCurrentAutoMovementSpeed) (.x _returnvalue_2)) (.y _returnvalue_2) (.z _returnvalue_2)) true true))
      (if (.bBlockingHit (Collision|BreakHitResult _sweephitresult)) ; If collision
        (if (Actor|ActorHasTag (.HitActor (Collision|BreakHitResult _sweephitresult)) "None") ; If obstacleTag
          _)))
    (:then_2
      ;[1 0.2684 0 1 47] GROUND DETECTION
      (bind (_outhit _returnvalue_4) (Class|KismetSystemLibrary|BoxTraceSingleforObjects _returnvalue_3 _returnvalue_3 "5.000000,5.000000,-2.000000" "0, 0, 0" (Utilities|Array|MakeArray "ObjectTypeQuery1") false 0 "None" true "(R=1.000000,G=0.000000,B=0.000000,A=1.000000)" "(R=0.000000,G=1.000000,B=0.000000,A=1.000000)" 0.0))
      (if _returnvalue_4 ; If touched something
        (if (Actor|ActorHasTag (.hitactor _outhit) "GroundBox")
          (if (not (Variables|Default|GetIsGrounded)) ; If I was airborne the frame before
            (CallFunction|LandingonGround)))
        (elif (Variables|Default|GetIsGrounded) ; If on the ground last frame
          (CallFunction|LeavingGround))))
    (:then_3
      (if (< (.z (Transformation|GetActorLocation)) -5e+02)
        (bind _returnvalue_5 (Game|GetCurrentLevelName true))
        (Game|OpenLevel(byName) (Utilities|String|StringToName _returnvalue_5))))))

(event Input|ActionEvents|InputActionDash
  (params (Key :type Key%20Structure :default "None"))
  (bind _returnvalue (Input|AxisValues|GetMoveForward))
  (bind _returnvalue_2 (Input|AxisValues|GetMoveRight))
  (bind _dashstrength (Variables|Default|GetDashStrength))
  (bind _returnvalue_3 (Math|Vector|MakeVector _returnvalue _returnvalue_2 0.0))
  (bind _returnvalue_4 (* _returnvalue_3 _dashstrength))
  ;[1 0.2937 0.9152 1 35] DASH
  (:Pressed
    (if (<= (Variables|Default|GetDashCooldownTimer) 0.0)
      (if (!= (Math|Vector|VectorLength _returnvalue_4) 0.0)
        (Character|LaunchCharacter _returnvalue_4 false false)
        (Variables|Default|SetDashCooldownTimer 15.0)))))

(event Input|ActionEvents|InputActionJump
  (params (Key :type Key%20Structure :default "None"))
  ;[0.0466 0.108 1 1 35] JUMP + BUFFERING + COYOTE TIME
  (:Pressed
    (if (or (Variables|Default|GetIsGrounded) (> (Variables|Default|GetCoyoteTimer) 0.0))
      (Character|Jump)
      (else
        (Variables|Default|SetJumpBufferingTimer 0.12)))))

(event Input|AxisEvents|InputAxisMoveForward
  (params (AxisValue :type Float%20%28single-precision%29))
  ;[0.07855 0.9103 1 1 45] MOVEMENT
  (Pawn|Input|AddMovementInput (Math|Vector|GetForwardVector (Variables|Collision|GetCapsuleComponent)) (* AxisValue (Variables|Default|GetMovementSpeed) (Utilities|Time|GetWorldDeltaSeconds) 0.3) false))

(event Input|AxisEvents|InputAxisMoveRight
  (params (AxisValue :type Float%20%28single-precision%29))
  (bind _returnvalue (Transformation|GetActorLocation))
  ;[0.07855 0.9103 1 1 45] MOVEMENT
  (Pawn|Input|AddMovementInput (Math|Vector|GetRightVector (Variables|Collision|GetCapsuleComponent)) (* AxisValue (Variables|Default|GetMovementSpeed) (Utilities|Time|GetWorldDeltaSeconds) 1.5) false)
  (Transformation|SetActorLocation (Math|Vector|MakeVector (.x _returnvalue) (Math|Float|Clamp(Float) (.y _returnvalue) -135.0 135.0) (.z _returnvalue)) false true))

(fn ConstructionScript)

(fn LandingonGround
  (if (> (Variables|Default|GetJumpBufferingTimer) 0.0) ; If Jump buffering enabled
    (Character|Jump)
    (Variables|Default|SetJumpBufferingTimer 0.0)
    (else
      (Variables|Default|SetIsGrounded true))))

(fn LeavingGround
  (Variables|Default|SetCoyoteTimer 0.15)
  (Variables|Default|SetIsGrounded false))